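; BP_BlueOfficer is an enemy character Blueprint whose own graph only visualizes its collision shapes for debugging.
; Every Tick, it draws boxes for its gun-fire and gun-bash collision components and a differently colored capsule for its body collision.
; The shapes follow each component's world transform and size, while BeginPlay, overlap and construction logic are empty.
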(event EventBeginPlay)

(event Collision|EventActorBeginOverlap
  (params (OtherActor :type Actor%20Object%20Reference)))

(event EventTick
  (params (DeltaSeconds :type Float%20%28single-precision%29))
  (bind _gunfirecollisionbox (Variables|Default|GetGunFireCollisionBox))
  (bind _gunbashcollisionbox (Variables|Default|GetGunBashCollisionBox))
  (bind _capsulecomponent (Variables|Default|GetCapsuleComponent))
  (Rendering|Debug|DrawDebugBox (Transformation|GetWorldLocation _gunfirecollisionbox) (Components|Box|GetScaledBoxExtent _gunfirecollisionbox) "(R=1.000000,G=0.100037,B=0.000000,A=1.000000)" (Transformation|GetWorldRotation _gunfirecollisionbox) 0.1 0.0)
  (Rendering|Debug|DrawDebugBox (Transformation|GetWorldLocation _gunbashcollisionbox) (Components|Box|GetScaledBoxExtent _gunbashcollisionbox) "(R=1.000000,G=0.100037,B=0.000000,A=1.000000)" (Transformation|GetWorldRotation _gunbashcollisionbox) 0.1 0.0)
  (Rendering|Debug|DrawDebugCapsule (Transformation|GetWorldLocation _capsulecomponent) (Variables|/Script/Engine.CapsuleComponent|GetCapsuleHalfHeight _capsulecomponent) (Components|Capsule|GetScaledCapsuleRadius _capsulecomponent) (Transformation|GetWorldRotation _capsulecomponent) "(R=0.000000,G=0.057555,B=1.000000,A=1.000000)" 0.0 2.0))

(fn ConstructionScript)